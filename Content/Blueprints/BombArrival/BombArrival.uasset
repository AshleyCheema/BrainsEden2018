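; BombArrival is an actor Blueprint that makes a bomb arrive at a random spot when a countdown runs out.
; Each Tick subtracts Timer from TimeRemaining and shuffles ObjectArray, which the graph does not otherwise use.
; At zero or below, a DoOnce moves the existing Bomb to a random point within the Box's bounds and stores the move's result in HasSpawned.
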(event `self.ReceiveBeginPlay`)

(event `self.ReceiveTick`
  (params (DeltaSeconds :type "Float (single-precision)"))
  (bind _box (`self.Box`))
  (`KismetArrayLibrary.Array_Shuffle` (`self.ObjectArray`))
  (bind _output_get (set `self.Time Remaining` (- (`self.Time Remaining`) (`self.Timer`))))
  (if (<= _output_get 0.0)
    (`/Engine/EditorBlueprintResources/StandardMacros.DoOnce` false
      (:`Completed`
        (bind (_sweephitresult _returnvalue) (`self.K2_SetActorLocation` (`self.Bomb`) (`KismetMathLibrary.RandomPointInBoundingBox` (`SceneComponent.K2_GetComponentLocation` _box) (`BoxComponent.BoxExtent` _box)) false false))
        (set `self.HasSpawned` _returnvalue)))))

(fn `UserConstructionScript`)