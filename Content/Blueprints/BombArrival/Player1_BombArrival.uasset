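; Player 1 bomb spawner that drops BombProjectile actors from random points inside its Box bounds.
; Tick runs a countdown, then shuffles ObjectArray and checks whether the first object's static mesh is hidden.
; If hidden, it reveals that mesh, spawns a projectile with downward velocity and resets the timer.
; If already visible, the timer stays expired, so the shuffle retries next tick.
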(event `self.ReceiveBeginPlay`)

(event `self.ReceiveTick`
  (params (DeltaSeconds :type "Float (single-precision)"))
  (bind _objectarray (`self.ObjectArray`))
  (bind _box (`self.Box`))
  ;[1 1 1] Timer for how long till the next bomb spawns
  (bind _output_get (set `self.Time Remaining` (- (`self.Time Remaining`) (`self.Timer`))))
  (if (<= _output_get 0.0)
    ;[1 1 1] Shuffles the array so it randomly drops different bombs. The bool is used to reference in the bomb object. Reset Timer
    (`KismetArrayLibrary.Array_Shuffle` _objectarray)
    (bind _output_get_2 (set `self.ObjectInArray` (`|GetArrayItem` _objectarray)))
    (bind _returnvalue (`self.GetComponentByClass` _output_get_2 "/Script/Engine.StaticMeshComponent"))
    (if (not (`SceneComponent.IsVisible` _returnvalue))
      (`SceneComponent.SetVisibility` _returnvalue true false)
      (bind _returnvalue_2 (`|SpawnActorFromClass` "/Game/JoshFo/BombProjectile.BombProjectile_C" (`KismetMathLibrary.Conv_VectorToTransform` (`KismetMathLibrary.RandomPointInBoundingBox` (`SceneComponent.K2_GetComponentLocation` _box) (`BoxComponent.BoxExtent` _box))) "Undefined" "OverrideRootScale" null null))
      (set `MovementComponent.Velocity` (0.0 0.0 -10.0) (`/Game/JoshFo/BombProjectile.ProjectileMovement` _returnvalue_2))
      (set `self.Time Remaining` 2.0))))

(fn `UserConstructionScript`)